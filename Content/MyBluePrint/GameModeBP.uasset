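; Game mode that spawns enemy waves from the GamePlayData table through a self-repeating SpawnLoop event, which nothing in this file starts.
; Each pass reads the row named by the loop counter, stores its scene and duration, and spawns enemies configured by per-index arrays for class, location, stats, movement and shooting.
; It then increments the counter, waits out the duration, clears the just-spawned list and repeats while rows exist.
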(event `SpawnLoop`
  (bind _returnvalue (`|GetDataTableRow` "/Game/MyBluePrint/GamePlayData.GamePlayData" (`KismetStringLibrary.Conv_StringToName` (`KismetStringLibrary.Conv_IntToString` (`self. SpawnLoopCounter`))))
    (:`then`
      (bind _output_get (set `self.CurrentRowData` _returnvalue))
      (bind (_seq _seqduration _scene _enemycount _actor _location _movement _health _movespeedmulti _xymulti _velocity _canshoot _firerate _projectile _scoregive) (break `/Game/MyBluePrint/GamePlayStruct` _output_get))
      (set `self.SpawnDelay` _seqduration)
      (set `self.Scene` _scene)
      (for _index (range _enemycount)
        (bind (_x _y) (`KismetMathLibrary.BreakVector2D` (`self.Safe_Get_Array_Element` _xymulti _index)))
        (bind _returnvalue_2 (`|SpawnActorFromClass` (`|GetArrayItem` (`self.EnemyClasses`) (`self.Safe_Get_Array_Element` _actor _index)) (`KismetMathLibrary.MakeTransform` (`self.Safe_Get_Array_Element` _location _index)) "Undefined" "OverrideRootScale" null (`self.Safe_Get_Array_Element` _health _index) (`self.Safe_Get_Array_Element` _scoregive _index) (`self.Safe_Get_Array_Element` _movement _index) (`self.Safe_Get_Array_Element` _movespeedmulti _index) _x _y (`self.Safe_Get_Array_Element` _velocity _index) (`self.Safe_Get_Array_Element` _canshoot _index) (`self.Safe_Get_Array_Element` _firerate _index) null null))
        (`KismetArrayLibrary.Array_AddUnique` (`self.EnemyJustSpawned`) _returnvalue_2))
      (bind _result (`/Engine/EditorBlueprintResources/StandardMacros.IncrementInt` (`self. SpawnLoopCounter`))
        (:`  `
          (set `self. SpawnLoopCounter` _result)
          (`KismetSystemLibrary.RetriggerableDelay` (`self.SpawnDelay`))
          (`KismetArrayLibrary.Array_Clear` (`self.EnemyJustSpawned`))
          (`self.SpawnLoop`))))))

(fn `UserConstructionScript`)